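; Automatic hitscan rifle that attaches to BP_ThirdPersonCharacter and pushes its ammo count to that player's HUD.
; A looping timer drives Shoot, which traces from the muzzle socket toward a point far along the camera's forward vector, with debug drawing.
; Hits apply point damage, spawn an explosion effect and briefly trigger an FS_MasterField actor at the impact.
; Reload waits on a retriggerable delay, adds ammo capped at MaxAmmo, then calls OnReloaded.
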(event `Equip`
  (bind _asbp_third_person_character (cast `/Game/ThirdPerson/Blueprints/BP_ThirdPersonCharacter` (`self.GetAttachParentActor`)))
  (set `self.Player` _asbp_third_person_character)
  (`self.UpdateHUD`))

(event `Reload`
  (params (Ammo :type Integer))
  (bind _returnvalue (+ Ammo (`self.Ammo`)))
  (`KismetSystemLibrary.RetriggerableDelay` 2.0)
  (if (> _returnvalue (`self.MaxAmmo`))
    (set `self.Ammo` (`self.MaxAmmo`))
    (else
      (set `self.Ammo` _returnvalue)))
  (`self.UpdateHUD`)
  (`self.OnReloaded` 0.0))

(event `StopShoot`
  (`KismetSystemLibrary.K2_ClearAndInvalidateTimerHandle` (`self.ShootTimer`)))

(event `StartShoot`
  (bind _returnvalue (`KismetSystemLibrary.K2_SetTimerDelegate` (delegate `Shoot`) (`self.FireRate`) true))
  (set `self.ShootTimer` _returnvalue)
  (`self.Shoot`))

(event `Shoot`
  (bind _returnvalue (`GameplayStatics.GetPlayerCameraManager` 0))
  (bind _returnvalue_2 (`SceneComponent.K2_GetComponentLocation` (`self.ShootSocket`)))
  (if (> (`self.Ammo`) 0)
    (`/Engine/EditorBlueprintResources/StandardMacros.DecrementInt` (`self.Ammo`)
      (:`  `
        (`self.UpdateHUD`)
        (bind _outhit (`KismetSystemLibrary.LineTraceSingleForObjects` _returnvalue_2 (+ (`PlayerCameraManager.GetCameraLocation` _returnvalue) (* (`self.GetActorForwardVector` _returnvalue) 20000)) (`|MakeArray` "ObjectTypeQuery1" "ObjectTypeQuery2" "ObjectTypeQuery3" :!type "EObjectTypeQuery Enum") false (`|MakeArray` (`self.GetAttachParentActor`)) "ForDuration" true (struct :`R` 1.0 :`A` 1.0) (struct :`G` 1.0 :`A` 1.0) 1.0))
        (`GameplayStatics.PlaySoundAtLocation` null _returnvalue_2 (struct) 1.0 1.0 0.0 null null null null)
        (bind (_bblockinghit _binitialoverlap _time _distance _location _impactpoint _normal _impactnormal _physmat _hitactor) (`GameplayStatics.BreakHitResult` _outhit))
        (if _bblockinghit
          (`self.Spawn Particles` _location (`KismetMathLibrary.MakeRotFromX` _normal))
          (`GameplayStatics.ApplyPointDamage` _hitactor 50.0 _location _outhit)
          (`self.SpawnMasterField` (`KismetMathLibrary.MakeTransform` _location)))))
    (else
      (`KismetSystemLibrary.PrintString` "Ammo empty!"))))

(event `Spawn Particles`
  (params (Location :type "Vector Structure") (Rotation :type "Rotator Structure"))
  (`GameplayStatics.SpawnEmitterAtLocation` "/Game/FPS_Weapon_Bundle/Weapons/FX/P_Explosion.P_Explosion" Location Rotation (`KismetMathLibrary.Conv_DoubleToVector` 0.5) true "AutoRelease"))

(event `SpawnMasterField`
  (params (SpawnTransform :type "Transform Structure"))
  (bind _returnvalue (`|SpawnActorFromClass` "/Engine/EditorResources/FieldNodes/FS_MasterField.FS_MasterField_C" SpawnTransform "Undefined" "OverrideRootScale" null null))
  (set `/Engine/EditorResources/FieldNodes/FS_MasterField.ActivationType` "NewEnumerator4" _returnvalue)
  (`/Engine/EditorResources/FieldNodes/FS_MasterField.CE_Trigger` _returnvalue)
  (`KismetSystemLibrary.Delay` 0.2)
  (`self.K2_DestroyActor` _returnvalue))

(fn `GetAmmo`
  (params (Current :type Boolean))
  (returns (Result :type Integer))
  (if Current
    (return (`self.Ammo`))
    (else
      (return (`self.MaxAmmo`)))))

(fn `UpdateHUD`
  (bind _player (`self.Player`))
  (`/Engine/EditorBlueprintResources/StandardMacros.IsValid` _player
    (:`Is Valid`
      (`/Game/UI/WBP_MainHUD.UpdateAmmoCount` (`/Game/ThirdPerson/Blueprints/BP_ThirdPersonCharacter.MainHUD` _player) (`self.Ammo`) (`self.MaxAmmo`)))))

(fn `UserConstructionScript`)