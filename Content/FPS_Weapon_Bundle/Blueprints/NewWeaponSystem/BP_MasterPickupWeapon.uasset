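; BP_MasterPickupWeapon is a weapon pickup, named as a master class, that the player can collect through interaction.
; Its PickupCollision overlap events set or clear the pickup as InteractionActor on the player's BP_ThirdPersonCharacter.
; Interact passes the weapon and socket to SpawnWeapons2 on the character reference cached at BeginPlay.
; The pickup destroys itself only if that spawn call succeeds.
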(event `self.PickupCollision.OnComponentBeginOverlap`
  (params (OverlappedComponent :type "PrimitiveComponent Object Reference") (OtherActor :type "Actor Object Reference") (OtherComp :type "PrimitiveComponent Object Reference") (OtherBodyIndex :type Integer) (bFromSweep :type Boolean) (SweepResult :type "HitResult Structure (by ref)"))
  (bind _returnvalue (`GameplayStatics.GetPlayerCharacter` 0))
  (if (== OtherActor _returnvalue)
    (bind _asbp_third_person_character (cast `/Game/ThirdPerson/Blueprints/BP_ThirdPersonCharacter` _returnvalue))
    (set `/Game/ThirdPerson/Blueprints/BP_ThirdPersonCharacter.InteractionActor` self _asbp_third_person_character)))

(event `self.PickupCollision.OnComponentEndOverlap`
  (params (OverlappedComponent :type "PrimitiveComponent Object Reference") (OtherActor :type "Actor Object Reference") (OtherComp :type "PrimitiveComponent Object Reference") (OtherBodyIndex :type Integer))
  (bind _returnvalue (`GameplayStatics.GetPlayerCharacter` 0))
  (if (== OtherActor _returnvalue)
    (bind _asbp_third_person_character (cast `/Game/ThirdPerson/Blueprints/BP_ThirdPersonCharacter` _returnvalue))
    (if (== (`/Game/ThirdPerson/Blueprints/BP_ThirdPersonCharacter.InteractionActor` _asbp_third_person_character) self)
      (set `/Game/ThirdPerson/Blueprints/BP_ThirdPersonCharacter.InteractionActor` null _asbp_third_person_character))))

(event `/Game/Common/BPI_Interact.Interact`
  (params (Player :type "Pawn Object Reference"))
  (bind _sucess (`/Game/ThirdPerson/Blueprints/BP_ThirdPersonCharacter.SpawnWeapons2` (`self.CharacterRef`) (`self.Weapons`) (`self.WeaponSocket`)))
  (if _sucess
    (`self.K2_DestroyActor`)))

(event `self.ReceiveBeginPlay`
  (bind _asbp_third_person_character (cast `/Game/ThirdPerson/Blueprints/BP_ThirdPersonCharacter` (`GameplayStatics.GetPlayerPawn` 0)))
  (set `self.CharacterRef` _asbp_third_person_character))

(fn `UserConstructionScript`)