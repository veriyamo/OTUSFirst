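; Core player controller that owns the main HUD, inventory toggling and player health and death.
; BeginPlay adds the inventory input mapping and creates the HUD; the inventory action and CloseInventory share a FlipFlop that slides the panel and switches input mode and cursor.
; Damage on the controller feeds its health component, with L and K keys applying test damage and healing (negative damage).
; Death plays a montage on the character, then quits the game on blend out.
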(event `self.ReceiveBeginPlay`
  (bind _returnvalue (pcsubsystem `EnhancedInputLocalPlayerSubsystem` self))
  (`/Engine/EditorBlueprintResources/StandardMacros.IsValid` _returnvalue
    (:`Is Valid`
      (`EnhancedInputSubsystemInterface.AddMappingContext` _returnvalue "/Game/ThirdPerson/Input/IMC_Inventory.IMC_Inventory" 0 (struct))
      (bind _returnvalue_2 (`|CreateWidget` "/Game/UI/WBP_MainHUD.WBP_MainHUD_C"))
      (bind _output_get (set `self.HUDRef` _returnvalue_2))
      (`UserWidget.AddToViewport` _output_get 0)
      (`WidgetBlueprintLibrary.SetInputMode_GameOnly` self)
      (set `self.bShowMouseCursor` false))))

(event `EnhancedInput|/Game/ThirdPerson/Input/Actions/IA_Inventory`
  (params (ActionValue :type Boolean) (ElapsedSeconds :type "Float (double-precision)") (TriggeredSeconds :type "Float (double-precision)") (InputAction :type "InputAction Object Reference" :default "/Game/ThirdPerson/Input/Actions/IA_Inventory.IA_Inventory"))
  (bind _hudref (`self.HUDRef`))
  (bind _slideinventory (`/Game/UI/WBP_MainHUD.SlideInventory` _hudref))
  (:`Started`
    (`/Engine/EditorBlueprintResources/StandardMacros.FlipFlop` :!label _label
      (:`A`
        (`WidgetBlueprintLibrary.SetInputMode_GameAndUIEx` self (`self.HUDRef`))
        (set `self.bShowMouseCursor` true)
        (`UserWidget.PlayAnimationForward` _hudref _slideinventory 1.0 false))
      (:`B`
        (`WidgetBlueprintLibrary.SetInputMode_GameOnly` self)
        (set `self.bShowMouseCursor` false)
        (`UserWidget.PlayAnimationReverse` _hudref _slideinventory 1.0 false)))))

(event `CloseInventory`
  (goto _label))

(event `Key|L`
  (params (Key :type "Key Structure"))
  (:`Pressed`
    (`GameplayStatics.ApplyDamage` self 20.0)))

(event `Key|K`
  (params (Key :type "Key Structure"))
  (:`Pressed`
    (`GameplayStatics.ApplyDamage` self -30.0)))

(event `self.ReceiveAnyDamage`
  (params (Damage :type "Float (single-precision)") (DamageType :type "DamageType Object Reference") (InstigatedBy :type "Controller Object Reference") (DamageCauser :type "Actor Object Reference"))
  (`/Game/Common/Components/BP_HealthComponent.OnHealthChange` (`self.BP_HealthComponent`) Damage))

(event `self.BP_HealthComponent.OnDead`
  (bind _asbp_third_person_character (cast `/Game/ThirdPerson/Blueprints/BP_ThirdPersonCharacter` (`GameplayStatics.GetPlayerCharacter` 0)))
  (`|PlayMontage` (`Character.Mesh` _asbp_third_person_character) "/Game/Characters/MainCharacter/Animations/AM_Death.AM_Death"
    (:`OnBlendOut`
      (`KismetSystemLibrary.QuitGame` null "Quit"))))

(fn `UserConstructionScript`)