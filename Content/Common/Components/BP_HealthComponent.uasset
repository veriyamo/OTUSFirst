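; Health component that tracks an owning actor's current health and signals when it dies.
; OnHealthChange takes a signed amount, treating positive values as healing capped at MaxHealth and other values as damage floored at zero.
; When damage brings health to zero or below, it calls OnDead.
; It does all its work in that function, with no BeginPlay or Tick logic.
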(fn `OnHealthChange`
  (params (Amount :type "Float (double-precision)"))
  (if (> Amount 0.0)
    ;[1 1 1] ToDoHeal
    (bind _output_get (set `self.CurrentHealth` (+ (`self.CurrentHealth`) (`local.Amount`))))
    (if (>= _output_get (`self.MaxHealth`))
      (set `self.CurrentHealth` (`self.MaxHealth`))
      (else
        (set `self.CurrentHealth` _output_get)))
    (else
      ;[1 1 1] ToDoDamage
      (bind _output_get_2 (set `self.CurrentHealth` (+ (`self.CurrentHealth`) (`local.Amount`))))
      (if (<= _output_get_2 0.0)
        (set `self.CurrentHealth` 0.0)
        (`self.OnDead`)
        (else
          (set `self.CurrentHealth` _output_get_2))))))